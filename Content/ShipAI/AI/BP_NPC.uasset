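; BP_NPC is an AI-controlled NPC pawn that seeds its controller's Blackboard when play begins.
; BeginPlay stores the pawn itself as SelfActor and sets HasPriority to true through the AI controller.
; An AIMoveTo node targeting the player character is left unconnected and never runs, and the construction script is empty.
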(event EventBeginPlay
  (bind _self self)
  (bind _returnvalue (AI|GetAIController _self))
  (bind _blackboard (Variables|/Script/AIModule.AIController|GetBlackboard _returnvalue))
  ;[0 1 1] Default values of SelfActor and HasPriority are set on the blackboard.
  (AI|Components|Blackboard|SetValueasObject _blackboard (Utilities|Name|MakeLiteralName "SelfActor") self)
  (AI|Components|Blackboard|SetValueasBool _blackboard (Utilities|Name|MakeLiteralName "HasPriority") true))

(fn ConstructionScript)