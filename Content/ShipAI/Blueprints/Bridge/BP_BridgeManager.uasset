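; Bridge manager that opens and closes the level's BP_Bridge for passing BP_NPC ships and drives its front and back signal lights.
; Overlaps on front and back collision boxes trigger it: an arriving ship sets that side's lights to seen, then opens the bridge after a random delay.
; On exit, an open, idle bridge closes if both boxes are empty; otherwise the empty side's lights show closed.
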(event OnComponentBeginOverlap(BridgeCollisionBack)
  (params (OverlappedComponent :type Primitive%20Component%20Object%20Reference) (OtherActor :type Actor%20Object%20Reference) (OtherComp :type Primitive%20Component%20Object%20Reference) (OtherBodyIndex :type Integer) (bFromSweep :type Boolean) (SweepResult :type Hit%20Result%20Structure%20%28by%20ref%29))
  ;[0 1 1] Ship enters collision
  (if (== (Utilities|GetClass OtherActor) "/Game/ShipAI/AI/BP_NPC.BP_NPC_C")
    (CallFunction|ShipEntersCollision false OtherActor)))

(event OnComponentBeginOverlap(BridgeCollisionFront)
  (params (OverlappedComponent :type Primitive%20Component%20Object%20Reference) (OtherActor :type Actor%20Object%20Reference) (OtherComp :type Primitive%20Component%20Object%20Reference) (OtherBodyIndex :type Integer) (bFromSweep :type Boolean) (SweepResult :type Hit%20Result%20Structure%20%28by%20ref%29))
  ;[0 1 1] Ship enters collision
  (if (== (Utilities|GetClass OtherActor) "/Game/ShipAI/AI/BP_NPC.BP_NPC_C")
    (CallFunction|ShipEntersCollision true OtherActor)))

(event OnComponentEndOverlap(BridgeCollisionFront)
  (params (OverlappedComponent :type Primitive%20Component%20Object%20Reference) (OtherActor :type Actor%20Object%20Reference) (OtherComp :type Primitive%20Component%20Object%20Reference) (OtherBodyIndex :type Integer))
  ;[0 1 1] Ship exits collision
  (CallFunction|ShipExitsCollision true OtherActor))

(event OnComponentEndOverlap(BridgeCollisionBack)
  (params (OverlappedComponent :type Primitive%20Component%20Object%20Reference) (OtherActor :type Actor%20Object%20Reference) (OtherComp :type Primitive%20Component%20Object%20Reference) (OtherBodyIndex :type Integer))
  ;[0 1 1] Ship exits collision
  (CallFunction|ShipExitsCollision false OtherActor))

(event Custom|ShipEntersCollision
  (params (Front? :type Boolean) (Ship :type Actor%20Object%20Reference))
  (bind _lightsback (Variables|Default|GetLightsBack))
  (bind _bridge (Variables|Default|GetBridge))
  (bind _lightsfront (Variables|Default|GetLightsFront))
  (bind _returnvalue (select Front? _lightsfront _lightsback))
  ;[0 1 1] If a ship enters the bridge collision, checks to see if the bridge is already open, opening, or closing, and the other collision box does NOT already contain this ship. If all of the criteria are met, it changes the lights to "Ship seen", gives it a random delay, and opens the bridge.
  (if (Math|Boolean|ANDBoolean (Math|Boolean|NORBoolean (Variables|/Game/ShipAI/Blueprints/Bridge/BP_Bridge.BP_Bridge_C|GetisOpening? _bridge) (Variables|/Game/ShipAI/Blueprints/Bridge/BP_Bridge.BP_Bridge_C|GetisClosing? _bridge)) (not (Variables|/Game/ShipAI/Blueprints/Bridge/BP_Bridge.BP_Bridge_C|GetisFullyOpen? _bridge)) (not (Utilities|Array|ContainsItem (Collision|GetOverlappingActors (select Front? (Variables|Default|GetBridgeCollisionBack) (Variables|Default|GetBridgeCollisionFront)) "/Game/ShipAI/AI/BP_NPC.BP_NPC_C" :!class /Script/Engine.PrimitiveComponent) Ship)))
    (for _array_element _returnvalue
      (Default|SetLights _array_element "NewEnumerator1"))
    (Utilities|FlowControl|Delay (Math|Random|RandomFloatinRange 1.0 1e+01))
    (Default|OpenorCloseBridge (Variables|Default|GetBridge) true _returnvalue)))

(event Custom|ShipExitsCollision
  (params (Front? :type Boolean) (Ship :type Actor%20Object%20Reference))
  (bind _bridge (Variables|Default|GetBridge))
  (bind _bridgecollisionfront (Variables|Default|GetBridgeCollisionFront))
  (bind _overlappingactors (Collision|GetOverlappingActors _bridgecollisionfront "/Game/ShipAI/AI/BP_NPC.BP_NPC_C" :!class /Script/Engine.PrimitiveComponent))
  (bind _returnvalue (Utilities|Array|IsEmpty _overlappingactors))
  ;[0 1 1] If a ship leaves the bridge collision box, checks if the bridge is currently open, and not in the process of opening or closing. Then checks to see if there are no more ships in either of the collision boxes. If this is true, the bridge closes. If there are still ships in the other collision box, the bridge is left open, but the lights are set to closed on the empty side.
  (if (and (Variables|/Game/ShipAI/Blueprints/Bridge/BP_Bridge.BP_Bridge_C|GetisFullyOpen? (Variables|Default|GetBridge)) (Math|Boolean|NORBoolean (Variables|/Game/ShipAI/Blueprints/Bridge/BP_Bridge.BP_Bridge_C|GetisOpening? _bridge) (Variables|/Game/ShipAI/Blueprints/Bridge/BP_Bridge.BP_Bridge_C|GetisClosing? _bridge)))
    (if (and (Utilities|Array|IsEmpty (Collision|GetOverlappingActors (Variables|Default|GetBridgeCollisionFront) "/Game/ShipAI/AI/BP_NPC.BP_NPC_C" :!class /Script/Engine.PrimitiveComponent)) (Utilities|Array|IsEmpty (Collision|GetOverlappingActors (Variables|Default|GetBridgeCollisionBack) "/Game/ShipAI/AI/BP_NPC.BP_NPC_C" :!class /Script/Engine.PrimitiveComponent)))
      (Default|OpenorCloseBridge (Variables|Default|GetBridge) false (select Front? (Variables|Default|GetLightsFront) (Variables|Default|GetLightsBack)))
      (elif (or _returnvalue (Utilities|Array|IsEmpty (Collision|GetOverlappingActors (Variables|Default|GetBridgeCollisionBack) "/Game/ShipAI/AI/BP_NPC.BP_NPC_C" :!class /Script/Engine.PrimitiveComponent)))
        (for _array_element (select _returnvalue (Variables|Default|GetLightsFront) (Variables|Default|GetLightsBack))
          (Default|SetLights _array_element "NewEnumerator0"))))))

(event EventBeginPlay
  ;[0 1 1] Sets the reference to bridge on begin play.
  (bind _returnvalue (Actor|GetActorOfClass "/Game/ShipAI/Blueprints/Bridge/BP_Bridge.BP_Bridge_C"))
  (Variables|Default|SetBridge _returnvalue))

(fn ConstructionScript)